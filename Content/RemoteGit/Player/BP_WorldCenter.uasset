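; BP_WorldCenter is the camera rig at the center of a ring-shaped play area, following the registered player.
; The construction script places arrows marking the ring's radii and camera reach, and sizes the spring arm.
; ActualiseCameraTransform converts the player's polar position into actor yaw and a clamped, remapped arm length.
; RegisterPlayer stores the player and enables Tick, which keeps the camera aimed at them.
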(event `self.ReceiveTick`
  (params (DeltaSeconds :type "Float (single-precision)"))
  (bind _returnvalue_location (`KismetMathLibrary.BreakTransform` (`self.GetTransform` (`self.Player Character`))))
  (`SceneComponent.K2_SetWorldRotation` (`self.Camera`) (`KismetMathLibrary.FindLookAtRotation` (`SceneComponent.K2_GetComponentLocation` (`self.Camera`)) _returnvalue_location) false false))

(fn `Actualise Camera Transform`
  (bind _totalradius (`self.TotalRadius`))
  (bind _output_get (set `self.Polar Plane` (`/Game/RemoteGit/Player/BP_PlayerCharacterBossFight.GetLocationAsPolar` (`self.Player Character`))))
  (bind (_x _y) (`KismetMathLibrary.BreakVector2D` _output_get))
  (`self.K2_SetActorRotation` (`KismetMathLibrary.MakeRotator` 0.0 0.0 _y))
  (set `SpringArmComponent.TargetArmLength` (`KismetMathLibrary.Sqrt` (+ (`KismetMathLibrary.Square` (`KismetMathLibrary.MapRangeClamped` _x (`self.Circl Start`) _totalradius (- _totalradius (`self.CameraReach`)) (+ (`self.TotalRadius`) 400.0))) (`KismetMathLibrary.Square` (`self.CameraPlayHeight`)))) (`self.SpringArm`)))

(fn `Register Player`
  (params (`Player character` :type "/Game/RemoteGit/Player/BP_PlayerCharacterBossFight Object Reference"))
  (set `self.Player Character` `Player character`)
  (`self.SetActorTickEnabled` true))

(fn `UserConstructionScript`
  (bind _output_get (set `self.TotalRadius` (+ (`self.Circl Start`) (`self.Circle Radius`))))
  (`SceneComponent.K2_SetRelativeLocation` (`self.ArrowOut`) (`KismetMathLibrary.MakeVector` _output_get 0.0 (`self.Z`)) false false)
  (`SceneComponent.K2_SetRelativeLocation` (`self.ArrowIn`) (`KismetMathLibrary.MakeVector` (`self.Circl Start`) 0.0 (`self.Z`)) false false)
  (`SceneComponent.K2_SetRelativeLocation` (`self.ArrowCamera`) (`KismetMathLibrary.MakeVector` (- (`self.TotalRadius`) (`self.CameraReach`)) 0.0 (`self.Z`)) false false)
  (set `SpringArmComponent.SocketOffset` (`KismetMathLibrary.MakeVector` 0.0 0.0 (`self.CameraPlayHeight`)) (`self.SpringArm`))
  (set `SpringArmComponent.TargetArmLength` (`KismetMathLibrary.Sqrt` (+ (`KismetMathLibrary.Square` (`self.TotalRadius`)) (`KismetMathLibrary.Square` (`self.CameraPlayHeight`)))) (`self.SpringArm`)))