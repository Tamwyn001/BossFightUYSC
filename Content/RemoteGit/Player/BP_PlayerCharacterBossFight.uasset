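; Player character Blueprint for boss fights, handling dash, roll, sword/bow swapping and walk effects, with stats, life and cooldown state kept on the PlayerController.
; Dash lerps location and camera FOV on a timeline with Niagara; roll launches the capsule with a montage while ignoring a collision channel.
; Montage notifies re-attach weapons between hand and back.
; Walk Niagara rate follows movement, falling and aiming; helper functions compute polar coordinates and quadrant.
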(event `self.ReceiveBeginPlay`
  (`SceneComponent.K2_SetWorldRotation` (`self.SpringArm`) (`KismetMathLibrary.MakeRotator` 0.0 0.0 60.0) false false))

(event `EnhancedInput|/Game/RemoteGit/Player/EnhancedInputs/IA_Move_Boss`
  (params (ActionValue :type "Vector2D Structure") (ElapsedSeconds :type "Float (double-precision)") (TriggeredSeconds :type "Float (double-precision)") (InputAction :type "InputAction Object Reference" :default "/Game/RemoteGit/Player/EnhancedInputs/IA_Move_Boss.IA_Move_Boss"))
  (:`Started`
    (`KismetSystemLibrary.RetriggerableDelay` 1.0)
    (`self.CheckNiagaraWalk`))
  (:`Canceled`
    (`self.CheckNiagaraWalk` :!label _label))
  (:`Completed`
    (goto _label)))

(event `self.ReceiveAnyDamage`
  (params (Damage :type "Float (single-precision)") (DamageType :type "DamageType Object Reference") (InstigatedBy :type "Controller Object Reference") (DamageCauser :type "Actor Object Reference"))
  (`/Game/RemoteGit/Player/BP_PlayControllerBossFight.UpdateLife` (`self.PlayerController`) (* (`KismetMathLibrary.FTrunc` Damage) -1)))

(event `EnhancedInput|/Game/RemoteGit/Player/EnhancedInputs/IA_Dash`
  (params (ActionValue :type Boolean) (ElapsedSeconds :type "Float (double-precision)") (TriggeredSeconds :type "Float (double-precision)") (InputAction :type "InputAction Object Reference" :default "/Game/RemoteGit/Player/EnhancedInputs/IA_Dash.IA_Dash"))
  (bind _returnvalue_location (`KismetMathLibrary.BreakTransform` (`self.GetTransform`)))
  (:`Started`
    (if (`/Game/RemoteGit/Player/BP_PlayControllerBossFight.Can DashOrRoll` (`self.PlayerController`))
      (set `/Game/RemoteGit/Player/BP_PlayControllerBossFight.Can DashOrRoll` false (`self.PlayerController`))
      (`|ExecutionSequence`
        (:`then_0`
          (set `self.DashStartLocation` _returnvalue_location)
          (set `self.DashEndLocation` (+ (* (`SceneComponent.GetForwardVector` (`self.CapsuleComponent`)) (`/Game/RemoteGit/Player/Stats/PDATA_PlayerStats.Dash Distance` (`/Game/RemoteGit/Player/BP_PlayControllerBossFight.Player Stats` (`self.PlayerController`)))) (`self.DashStartLocation`)))
          (`TimelineComponent.SetPlayRate` (`self.Dash`) 3.0)
          (set `self.BeginFOV` (`/Game/RemoteGit/Player/BP_PlayControllerBossFight.GetCameraFOV` (`self.PlayerController`)))
          (bind (_direction _alpha _camerafovalpha) (`Timeline|Dash` :!via `PlayFromStart`)
            (:`Update`
              (`self.K2_SetActorLocation` (`KismetMathLibrary.VLerp` (`self.DashStartLocation`) (`self.DashEndLocation`) _alpha))
              (`/Game/RemoteGit/Player/BP_PlayControllerBossFight.UpdateCameraFOV` (`self.PlayerController`) (`KismetMathLibrary.Lerp` (`self.BeginFOV`) 91.0 _camerafovalpha)))
            (:`Finished`
              (`KismetSystemLibrary.Delay` (`/Game/RemoteGit/Player/Stats/PDATA_PlayerStats.Roll Immunity Duration` (`/Game/RemoteGit/Player/BP_PlayControllerBossFight.Player Stats` (`self.PlayerController`))))
              (set `/Game/RemoteGit/Player/BP_PlayControllerBossFight.Can DashOrRoll` true (`self.PlayerController`)))))
        (:`then_1`
          (`NiagaraFunctionLibrary.SpawnSystemAttached` "/Game/RemoteGit/Niagara/NS_Dash.NS_Dash" (`self.Mesh`) "None" (0.0 0.0 0.0) (struct) "KeepRelativeOffset" true))))))

(event `EnhancedInput|/Game/RemoteGit/Player/EnhancedInputs/IA_Roll`
  (params (ActionValue :type Boolean) (ElapsedSeconds :type "Float (double-precision)") (TriggeredSeconds :type "Float (double-precision)") (InputAction :type "InputAction Object Reference" :default "/Game/RemoteGit/Player/EnhancedInputs/IA_Roll.IA_Roll"))
  (bind _playercontroller (`self.PlayerController`))
  (:`Started`
    (if (not (or (not (`/Game/RemoteGit/Player/BP_PlayControllerBossFight.Can DashOrRoll` _playercontroller)) (`NavMovementComponent.IsFalling` (`self.CharacterMovement`)) false))
      (set `/Game/RemoteGit/Player/BP_PlayControllerBossFight.Can DashOrRoll` false _playercontroller)
      (`PrimitiveComponent.SetCollisionResponseToChannel` (`self.CapsuleComponent`) "ECC_GameTraceChannel1" "ECR_Ignore")
      (`self.LaunchCharacter` (* (`SceneComponent.GetForwardVector` (`self.CapsuleComponent`)) (`/Game/RemoteGit/Player/Stats/PDATA_PlayerStats.Roll Distance` (`/Game/RemoteGit/Player/BP_PlayControllerBossFight.Player Stats` _playercontroller))))
      (`|PlayMontage` (`self.Mesh`) "/Game/RemoteGit/Player/AnimsBPs/MONTAGE_Sprinting_Forward_Roll.MONTAGE_Sprinting_Forward_Roll"
        (:`OnCompleted`
          (set `/Game/RemoteGit/Player/BP_PlayControllerBossFight.Can DashOrRoll` true (`self.PlayerController`))
          (`PrimitiveComponent.SetCollisionResponseToChannel` (`self.CapsuleComponent`) "ECC_GameTraceChannel1" "ECR_Overlap"))))))

(event `self.OnLanded`
  (params (Hit :type "HitResult Structure (by ref)"))
  (`self.CheckNiagaraWalk`))

(event `self.OnLaunched`
  (params (LaunchVelocity :type "Vector Structure") (bXYOverride :type Boolean) (bZOverride :type Boolean))
  (`self.CheckNiagaraWalk`))

(event `AnimBowToBack`
  (`SceneComponent.K2_AttachToComponent` (`self.MeshBow`) (`self.BackBowScene`) "None" "KeepRelative" "KeepRelative" "KeepRelative" true)
  (`KismetSystemLibrary.MoveComponentTo` (`self.MeshBow`) (0.0 0.0 0.0) (struct) false false 0.2 true))

(event `MoveSwordToBack`
  (`SceneComponent.K2_AttachToComponent` (`self.MeshSword`) (`self.BackSwordScene`) "None" "KeepRelative" "KeepRelative" "KeepRelative" true)
  (`KismetSystemLibrary.MoveComponentTo` (`self.MeshSword`) (0.0 0.0 0.0) (struct) false false 0.2 true))

(event `AnimBowToHand`
  (`SceneComponent.K2_AttachToComponent` (`self.MeshBow`) (`self.BowScene`) "None" "KeepRelative" "KeepRelative" "KeepRelative" true)
  (`KismetSystemLibrary.MoveComponentTo` (`self.MeshBow`) (0.0 0.0 0.0) (struct) false false 0.2 true))

(event `MoveSwordToHand`
  (`SceneComponent.K2_AttachToComponent` (`self.MeshSword`) (`self.SwordScene`) "None" "KeepRelative" "KeepRelative" "KeepRelative" true)
  (`KismetSystemLibrary.MoveComponentTo` (`self.MeshSword`) (0.0 0.0 0.0) (struct) false false 0.2 true))

(event `DrawSwordToBow`
  (bind _notifyname (`|PlayMontage` (`self.Mesh`) "/Game/RemoteGit/Player/AnimsBPs/MONATGE_BackSword.MONATGE_BackSword")
    (:`OnCompleted`
      (`/Game/RemoteGit/Player/BP_PlayControllerBossFight.Reload arrow` (`self.PlayerController`)))
    (:`OnNotifyBegin`
      (if (== _notifyname "SwordBack")
        (`self.MoveSwordToBack`)
        (bind _notifyname_2 (`|PlayMontage` (`self.Mesh`) "/Game/RemoteGit/Player/AnimsBPs/MONATGE_OutBow.MONATGE_OutBow")
          (:`OnInterrupted`
            (`KismetSystemLibrary.PrintString` "Inter"))
          (:`OnNotifyBegin`
            (if (== _notifyname_2 "Transfer")
              (`self.AnimBowToHand`)
              (`KismetSystemLibrary.PrintString` "transd")
              (set `/Game/RemoteGit/Player/AnimsBPs/AnimBP_Hero.BowEquiped` true (`/Game/RemoteGit/Player/BP_PlayControllerBossFight.AnimInstancePlayer` (`self.PlayerController`))))))))))

(event `DrawBowToSword`
  (bind _notifyname (`|PlayMontage` (`self.Mesh`) "/Game/RemoteGit/Player/AnimsBPs/MONTAGE_BowBack.MONTAGE_BowBack")
    (:`OnNotifyBegin`
      (if (== _notifyname "BowBack")
        (`self.AnimBowToback`)
        (set `/Game/RemoteGit/Player/AnimsBPs/AnimBP_Hero.BowEquiped` false (`/Game/RemoteGit/Player/BP_PlayControllerBossFight.AnimInstancePlayer` (`self.PlayerController`)))
        (bind _notifyname_2 (`|PlayMontage` (`self.Mesh`) "/Game/RemoteGit/Player/AnimsBPs/MONATGE_OutSword.MONATGE_OutSword")
          (:`OnNotifyBegin`
            (if (== _notifyname_2 "Transfer")
              (`self.MoveSwordToHand`))))))))

(event `InputVectorAxis|Gamepad_Left2D`
  (params (AxisValue :type "Vector Structure"))
  (`KismetSystemLibrary.PrintString` (`KismetStringLibrary.Conv_VectorToString` AxisValue)))

(fn `CheckNiagaraWalk`
  (if (or (== (`|GetInputActionValue`) (0.0 0.0)) (`NavMovementComponent.IsFalling` (`self.CharacterMovement`)))
    (`FXSystemComponent.SetFloatParameter` (`self.WalkNiagara`) "user.rate" 0.0)
    (else
      (`|ExecutionSequence`
        (:`then_0`
          (`/Engine/EditorBlueprintResources/StandardMacros.IsValid` (`self.WalkNiagara`)
            (:`Is Not Valid`
              (bind _returnvalue (`NiagaraFunctionLibrary.SpawnSystemAttached` "/Game/RemoteGit/Niagara/NS_Walk.NS_Walk" (`self.Mesh`) "None" (0.0 0.0 0.0) (struct) "KeepRelativeOffset"))
              (set `self.WalkNiagara` _returnvalue))))
        (:`then_1`
          (`FXSystemComponent.SetFloatParameter` (`self.WalkNiagara`) "user.rate" (`KismetMathLibrary.SelectFloat` 1.0 10.0 (`/Game/RemoteGit/Player/BP_PlayControllerBossFight.Is Aiming` (`self.PlayerController`)))))))))

(fn `Get Cartesian Coordinates`
  (params (RadiusAngle :type "Vector2D Structure"))
  (returns (XY :type "Vector2D Structure"))
  (bind (_x _y) (`KismetMathLibrary.BreakVector2D` RadiusAngle))
  (return (`KismetMathLibrary.MakeVector2D` (* _x (`KismetMathLibrary.DegCos` _y)) (* _x (`KismetMathLibrary.DegSin` _y)))))

(fn `Get PolarCoordinates`
  (params (XY :type "Vector2D Structure"))
  (returns (RadiusAngle :type "Vector2D Structure"))
  (bind (_x _y) (`KismetMathLibrary.BreakVector2D` XY))
  (return (`KismetMathLibrary.MakeVector2D` (`KismetMathLibrary.Sqrt` (+ (`KismetMathLibrary.Square` _x) (`KismetMathLibrary.Square` _y))) (`KismetMathLibrary.DegAtan` (/ _x _y)))))

(fn `Get quadrant`
  (returns (QuadrantID :type Integer))
  (bind (_returnvalue_x _returnvalue_y) (`KismetMathLibrary.BreakVector` (`self.K2_GetActorLocation`)))
  (return (`KismetMathLibrary.SelectInt` 0 (`KismetMathLibrary.SelectInt` 2 (`KismetMathLibrary.SelectInt` 1 3 (<= _returnvalue_x 0.0)) (and (<= _returnvalue_x 0.0) (<= _returnvalue_y 0.0))) (and (> _returnvalue_x 0.0) (> _returnvalue_y 0.0)))))

(fn `GetLocationAsPolar`
  (returns (PolarPlane :type "Vector2D Structure"))
  (bind (_x _y) (`KismetMathLibrary.BreakVector2D` (`KismetMathLibrary.Conv_VectorToVector2D` (`self.K2_GetActorLocation`))))
  (return (`KismetMathLibrary.MakeVector2D` (`KismetMathLibrary.Sqrt` (+ (`KismetMathLibrary.Square` _x) (`KismetMathLibrary.Square` _y))) (`KismetMathLibrary.DegAtan2` _y _x))))

(fn `UserConstructionScript`)