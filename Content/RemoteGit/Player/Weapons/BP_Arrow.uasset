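; BP_Arrow is a weapon projectile actor for an arrow, launched at a SpawnVelocity and destroyed after a fixed lifetime.
; On BeginPlay it turns on physics simulation for its StaticMesh, makes the mesh ignore the player pawn when moving, and sets the ProjectileMovement velocity in local space.
; Mesh hit and projectile bounce events only print the name of the actor struck, with no damage or other impact logic.
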(event `self.ReceiveBeginPlay`
  (`PrimitiveComponent.SetSimulatePhysics` (`self.StaticMesh`) true)
  (`PrimitiveComponent.IgnoreActorWhenMoving` (`self.StaticMesh`) (`GameplayStatics.GetPlayerPawn` 0) true)
  (`ProjectileMovementComponent.SetVelocityInLocalSpace` (`self.ProjectileMovement`) (`self.SpawnVelocity`))
  (`KismetSystemLibrary.Delay` 7.0)
  (`self.K2_DestroyActor`))

(event `self.StaticMesh.OnComponentHit`
  (params (HitComponent :type "PrimitiveComponent Object Reference") (OtherActor :type "Actor Object Reference") (OtherComp :type "PrimitiveComponent Object Reference") (NormalImpulse :type "Vector Structure") (Hit :type "HitResult Structure (by ref)"))
  (`KismetSystemLibrary.PrintString` (`KismetSystemLibrary.GetDisplayName` OtherActor)))

(event `self.ProjectileMovement.OnProjectileBounce`
  (params (ImpactResult :type "HitResult Structure (by ref)") (ImpactVelocity :type "Vector Structure (by ref)"))
  (`KismetSystemLibrary.PrintString` (`KismetSystemLibrary.GetDisplayName` (`.HitActor` (`GameplayStatics.BreakHitResult` ImpactResult)))))

(fn `UserConstructionScript`)