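; Player controller for the boss fight, handling Enhanced Input, life and arrow counts, and the main HUD.
; Movement follows the active camera, either the character's or a registered WorldCenter arena camera, with BPCCameraDrag receiving look input.
; Jump height scales with hold time through a curve.
; Bow aiming slows and turns the player toward the cursor; montage notifies spawn and fire arced arrows, while sword attack only runs a cooldown.
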(event `EnhancedInput|/Game/RemoteGit/Player/EnhancedInputs/IA_MoveCameraEnabled`
  (params (ActionValue :type Boolean) (ElapsedSeconds :type "Float (double-precision)") (TriggeredSeconds :type "Float (double-precision)") (InputAction :type "InputAction Object Reference" :default "/Game/RemoteGit/Player/EnhancedInputs/IA_MoveCameraEnabled.IA_MoveCameraEnabled"))
  (bind _player_stats (`self.Player Stats`))
  (bind _as_bp_player_character_boss_fight (`self.As BP Player Character Boss Fight`))
  (bind _walkniagara (`/Game/RemoteGit/Player/BP_PlayerCharacterBossFight.WalkNiagara` _as_bp_player_character_boss_fight))
  (:`Started`
    (switch `/Game/RemoteGit/Player/Weapons/E_Weapon` (`self.EquipedWepon`)
      (:`NewEnumerator0`
        (set `self.Is Aiming` true)
        (set `CharacterMovementComponent.bOrientRotationToMovement` false (`Character.CharacterMovement` (`self.As BP Player Character Boss Fight`)))
        (`FXSystemComponent.SetFloatParameter` _walkniagara "user.rate" 1.0)
        (bind (_direction _speedalpha) (`Timeline|AimSlow` :!via `PlayFromStart` :!label _label)
          (:`Update`
            (set `CharacterMovementComponent.MaxWalkSpeed` (`KismetMathLibrary.Lerp` (`/Game/RemoteGit/Player/Stats/PDATA_PlayerStats.RunSpeed` _player_stats) (`/Game/RemoteGit/Player/Stats/PDATA_PlayerStats.AimSpeed` _player_stats) _speedalpha) (`Character.CharacterMovement` (`self.As BP Player Character Boss Fight`))))))))
  (:`Canceled`
    (set `self.Is Aiming` false :!label _label_2)
    (set `CharacterMovementComponent.bOrientRotationToMovement` true (`Character.CharacterMovement` (`self.As BP Player Character Boss Fight`)))
    (`FXSystemComponent.SetFloatParameter` _walkniagara "user.rate" 10.0)
    (`/Game/RemoteGit/Player/BP_PlayerCharacterBossFight.CheckNiagaraWalk` _as_bp_player_character_boss_fight)
    (goto _label :!via `Reverse`))
  (:`Completed`
    (goto _label_2)))

(event `EnhancedInput|/Game/RemoteGit/Player/EnhancedInputs/IA_ChangeWeapon`
  (params (ActionValue :type Boolean) (ElapsedSeconds :type "Float (double-precision)") (TriggeredSeconds :type "Float (double-precision)") (InputAction :type "InputAction Object Reference" :default "/Game/RemoteGit/Player/EnhancedInputs/IA_ChangeWeapon.IA_ChangeWeapon"))
  (:`Started`
    (switch `/Game/RemoteGit/Player/Weapons/E_Weapon` (`self.EquipedWepon`)
      (:`NewEnumerator0`
        (set `self.ArrowEquiped` false)
        (`self.K2_AttachToComponent` (`self.AsArrowEquiped`) (`/Game/RemoteGit/Player/BP_PlayerCharacterBossFight.SwordScene` (`self.As BP Player Character Boss Fight`)) "None" "SnapToTarget" "SnapToTarget" "KeepWorld" true)
        (`self.K2_AddActorLocalRotation` (`self.AsArrowEquiped`) (struct :`Yaw` 90.0) false false)
        (`self.K2_AddActorLocalOffset` (30.0 0.0 0.0))
        (bind _notifyname (`|PlayMontage` (`Character.Mesh` (`GameplayStatics.GetPlayerCharacter` 0)) "/Game/RemoteGit/Player/AnimsBPs/MONTAGE_UnEquip_Arrow.MONTAGE_UnEquip_Arrow")
          (:`OnBlendOut`
            (`self.ChangeSelected weapon` "NewEnumerator1"))
          (:`OnNotifyBegin`
            (if (== _notifyname "KillArrow")
              (`self.K2_DestroyActor` (`self.AsArrowEquiped`))
              (set `self.AsArrowEquiped` null)))))
      (:`NewEnumerator1`
        (`self.ChangeSelected weapon` "NewEnumerator0")))))

(event `EnhancedInput|/Game/RemoteGit/Player/EnhancedInputs/IA_Move_Boss`
  (params (ActionValue :type "Vector2D Structure") (ElapsedSeconds :type "Float (double-precision)") (TriggeredSeconds :type "Float (double-precision)") (InputAction :type "InputAction Object Reference" :default "/Game/RemoteGit/Player/EnhancedInputs/IA_Move_Boss.IA_Move_Boss"))
  (bind _world_center (`self.World Center`))
  (bind (_returnvalue_location _returnvalue_rotation) (`KismetMathLibrary.BreakTransform` (`self.GetTransform` _world_center)))
  (:`Triggered`
    (`self.InputMovment` ActionValue))
  (:`Started`
    (`|ExecutionSequence`
      (:`then_0`
        (if (`self.CameraCenterRegistered`)
          (set `self.StartRotatorFollow` (`KismetMathLibrary.NormalizedDeltaRotator` _returnvalue_rotation (struct :`Yaw` 180.0)))
          (`TimelineComponent.SetPlayRate` (`self.CameraStartFollow`) 1.4)
          (bind (_direction _alpha) (`Timeline|CameraStartFollow` :!via `PlayFromStart`)
            (:`Update`
              (`SceneComponent.K2_SetWorldRotation` (`/Game/RemoteGit/Player/BP_WorldCenter.SpringArm` _world_center) (`KismetMathLibrary.RLerp` (`self.StartRotatorFollow`) (`KismetMathLibrary.NormalizedDeltaRotator` _returnvalue_rotation (struct :`Yaw` 180.0)) _alpha) false false)))))
      (:`then_1`
        (bind (_direction_2 _alpha_2) (`Timeline|Walk` :!via `PlayFromStart` :!label _label_3)
          (:`Update`
            (`self.UpdateCameraFOV` (`KismetMathLibrary.Lerp` 88.0 90.0 _alpha_2)))))))
  (:`Canceled`
    (goto _label_3 :!via `Reverse`))
  (:`Completed`
    (goto _label_3 :!via `Reverse`)))

(event `self.ReceiveBeginPlay`
  (bind _returnvalue (`GameplayStatics.GetPlayerController` 0))
  (set `self.CurrentLife` (`/Game/RemoteGit/Player/Stats/PDATA_PlayerStats.MaxHealth` (`self.Player Stats`)))
  (`|ExecutionSequence`
    (:`then_0`
      (`EnhancedInputSubsystemInterface.AddMappingContext` (pcsubsystem `EnhancedInputLocalPlayerSubsystem` (`GameplayStatics.GetPlayerController` 0)) "/Game/RemoteGit/Player/EnhancedInputs/IMC_BossFight.IMC_BossFight" 0 (make `ModifyContextOptions` true))
      (bind _asbp_player_character_boss_fight (cast `/Game/RemoteGit/Player/BP_PlayerCharacterBossFight` (`GameplayStatics.GetPlayerCharacter` 0)))
      (bind _output_get (set `self.As BP Player Character Boss Fight` _asbp_player_character_boss_fight))
      (set `/Game/RemoteGit/Player/BP_PlayerCharacterBossFight.PlayerController` self _output_get)
      (`/Game/RemoteGit/Player/BPC_CameraDrag.Register New camera` (`self.BPC_CameraDrag`) (`/Game/RemoteGit/Player/BP_PlayerCharacterBossFight.Camera` _output_get))
      (set `CharacterMovementComponent.MaxWalkSpeed` (`/Game/RemoteGit/Player/Stats/PDATA_PlayerStats.RunSpeed` (`self.Player Stats`)) (`Character.CharacterMovement` (`self.As BP Player Character Boss Fight`)))
      (bind _returnvalue_2 (`|CreateWidget` "/Game/RemoteGit/Widgets/Widget_Main.Widget_Main_C" null self))
      (bind _output_get_2 (set `self.Main Widget` _returnvalue_2))
      (`UserWidget.AddToViewport` _output_get_2 0)
      (bind _asanim_bp_hero (cast `/Game/RemoteGit/Player/AnimsBPs/AnimBP_Hero` (`SkeletalMeshComponent.GetAnimInstance` (`Character.Mesh` (`self.As BP Player Character Boss Fight`)))))
      (set `self.AnimInstancePlayer` _asanim_bp_hero))
    (:`then_1`
      (`KismetSystemLibrary.ExecuteConsoleCommand` "r.DynamicGlobalIlluminationMethod 0" _returnvalue)
      (`KismetSystemLibrary.ExecuteConsoleCommand` "r.AntiAliasingMethod 3" _returnvalue))
    (:`then_2`
      (`self.InitArrows`))))

(event `self.ReceiveTick`
  (params (DeltaSeconds :type "Float (single-precision)"))
  (bind _player_stats (`self.Player Stats`))
  (bind (_aimingrotator_roll _aimingrotator_pitch _aimingrotator_yaw) (`KismetMathLibrary.BreakRotator` (`self.AimingRotator`)))
  (bind _returnvalue_location (`KismetMathLibrary.BreakTransform` (`self.GetTransform` (`self.As BP Player Character Boss Fight`))))
  (bind _jumpheight (`/Game/RemoteGit/Player/Stats/PDATA_PlayerStats.JumpHeight` _player_stats))
  (bind _maxjumptime (`/Game/RemoteGit/Player/Stats/PDATA_PlayerStats.MaxJumpTime` _player_stats))
  (`|ExecutionSequence`
    (:`then_0`
      (if (`self.Is Aiming`)
        (bind _output_get (set `self.AimingLocation` (`.Location` (`GameplayStatics.BreakHitResult` (`self.GetHitResultUnderCursorByChannel` "TraceTypeQuery1")))))
        (set `self.AimingRotator` (`KismetMathLibrary.FindLookAtRotation` (+ _returnvalue_location (0.0 0.0 120.0)) _output_get))
        (`KismetSystemLibrary.DrawDebugSphere` _output_get 50.0 12 (struct :`R` 1.0 :`G` 1.0 :`B` 1.0 :`A` 1.0) 0.0 10.0)
        (`self.K2_SetActorRotation` (`self.As BP Player Character Boss Fight`) (`KismetMathLibrary.MakeRotator` 0.0 0.0 _aimingrotator_yaw) false)))
    (:`then_1`
      (if (`self.Jump Pressed`)
        (`/Game/RemoteGit/Widgets/Widget_Main.Update Jump Time` (`self.Main Widget`) (/ (`CurveFloat.GetFloatValue` _jumpheight (/ (`KismetMathLibrary.FClamp` (`self.JumpTimePressed`) 0.0 _maxjumptime) _maxjumptime)) (`.MaxValue` (`CurveBase.GetValueRange` _jumpheight))))
        (set `self.JumpTimePressed` (+ (`self.JumpTimePressed`) (`GameplayStatics.GetWorldDeltaSeconds`)))))))

(event `EnhancedInput|/Game/RemoteGit/Player/EnhancedInputs/IA_Jump_Boss`
  (params (ActionValue :type Boolean) (ElapsedSeconds :type "Float (double-precision)") (TriggeredSeconds :type "Float (double-precision)") (InputAction :type "InputAction Object Reference" :default "/Game/RemoteGit/Player/EnhancedInputs/IA_Jump_Boss.IA_Jump_Boss"))
  (bind _player_stats (`self.Player Stats`))
  (bind _maxjumptime (`/Game/RemoteGit/Player/Stats/PDATA_PlayerStats.MaxJumpTime` _player_stats))
  (:`Started`
    (if (not (`self.IsPlayerFalling`))
      (`/Game/RemoteGit/Widgets/Widget_Main.Jump Started` (`self.Main Widget`))
      (set `self.JumpTimePressed` 0.0)
      (set `self.Jump Pressed` true)))
  (:`Canceled`
    (`/Game/RemoteGit/Widgets/Widget_Main.Jump finished` (`self.Main Widget`) :!label _label_4)
    (set `self.Jump Pressed` false)
    (if (not (`self.IsPlayerFalling`))
      (`Character.LaunchCharacter` (`self.As BP Player Character Boss Fight`) (`KismetMathLibrary.MakeVector` 0.0 0.0 (`CurveFloat.GetFloatValue` (`/Game/RemoteGit/Player/Stats/PDATA_PlayerStats.JumpHeight` _player_stats) (/ (`KismetMathLibrary.FClamp` ElapsedSeconds 0.0 _maxjumptime) _maxjumptime))) false false)))
  (:`Completed`
    (goto _label_4)))

(event `On Arrow Land`
  (`/Game/RemoteGit/Player/BPC_CameraDrag.Arrow Reached` (`self.BPC_CameraDrag`)))

(event `Move Arrow to bow`
  (bind _asarrowequiped (`self.AsArrowEquiped`))
  (`SceneComponent.K2_AttachToComponent` (`/Game/RemoteGit/Player/Weapons/BP_Arrow.StaticMesh` _asarrowequiped) (`/Game/RemoteGit/Player/BP_PlayerCharacterBossFight.MeshBow` (`self.As BP Player Character Boss Fight`)) "None" "SnapToTarget" "KeepRelative" "KeepRelative" true)
  (`self.K2_AddActorLocalRotation` (`self.AsArrowEquiped`) (struct :`Yaw` 180.0) false false)
  (`self.K2_AddActorLocalOffset` _asarrowequiped (20.0 0.0 0.0) false false))

(event `EnhancedInput|/Game/RemoteGit/Player/EnhancedInputs/IA_Attack`
  (params (ActionValue :type Boolean) (ElapsedSeconds :type "Float (double-precision)") (TriggeredSeconds :type "Float (double-precision)") (InputAction :type "InputAction Object Reference" :default "/Game/RemoteGit/Player/EnhancedInputs/IA_Attack.IA_Attack"))
  (bind _returnvalue_location (`KismetMathLibrary.BreakTransform` (`self.GetTransform` (`self.AsArrowEquiped`))))
  (:`Started`
    (if (`self.Can attack`)
      (switch `/Game/RemoteGit/Player/Weapons/E_Weapon` (`self.EquipedWepon`)
        (:`NewEnumerator0`
          (if (`self.ArrowEquiped`)
            (set `self.Can attack` false)
            (`self.Update Arrows` -1)
            (bind _notifyname (`|PlayMontage` (`Character.Mesh` (`GameplayStatics.GetPlayerCharacter` 0)) "/Game/RemoteGit/Player/AnimsBPs/MONTAGE_BowShoot.MONTAGE_BowShoot")
              (:`then`
                (set `self.ArrowEquiped` false))
              (:`OnBlendOut`
                (if (> (`self.Arrows`) 0)
                  (`self.Reload arrow`)))
              (:`OnNotifyBegin`
                (if (== _notifyname "Shoot")
                  (bind _outlaunchvelocity (`GameplayStatics.SuggestProjectileVelocity_CustomArc` _returnvalue_location (`.Location` (`GameplayStatics.BreakHitResult` (`self.GetHitResultUnderCursorByChannel` "TraceTypeQuery1"))) 0.0 0.8))
                  (bind _returnvalue (`|SpawnActorFromClass` "/Game/RemoteGit/Player/Weapons/BP_Arrow.BP_Arrow_C" (`KismetMathLibrary.MakeTransform` _returnvalue_location) "Undefined" "MultiplyWithRoot" null _outlaunchvelocity null))
                  (`/Game/RemoteGit/Player/BPC_CameraDrag.Register Arrow shoot` (`self.BPC_CameraDrag`))
                  (`self.K2_DestroyActor` (`self.AsArrowEquiped`))
                  (`/Game/RemoteGit/Player/Weapons/BP_Arrow.Shoot` _returnvalue))))))
        (:`NewEnumerator1`
          (set `self.Can attack` false)
          (`KismetSystemLibrary.Delay` (`/Game/RemoteGit/Player/Stats/PDATA_PlayerStats.AttackDelay` (`self.Player Stats`)))
          (set `self.Can attack` true))))))

(event `Reload arrow`
  (bind _returnvalue_location (`KismetMathLibrary.BreakTransform` (`self.GetTransform` (`self.As BP Player Character Boss Fight`))))
  (bind _notifyname (`|PlayMontage` (`Character.Mesh` (`GameplayStatics.GetPlayerCharacter` 0)) "/Game/RemoteGit/Player/AnimsBPs/MONTAGE_Equip_Arrow.MONTAGE_Equip_Arrow")
    (:`OnCompleted`
      (set `self.Can attack` true)
      (if (not (`self.Is Aiming`))
        (`self.Move Arrow to bow`)))
    (:`OnBlendOut`
      (if (`self.Is Aiming`)
        (`self.Move Arrow to bow`)))
    (:`OnNotifyBegin`
      (if (== _notifyname "DrawArrow")
        (set `self.ArrowEquiped` true)
        (bind _returnvalue (`|SpawnActorFromClass` "/Game/RemoteGit/Player/Weapons/BP_Arrow.BP_Arrow_C" (`KismetMathLibrary.MakeTransform` _returnvalue_location (struct) (0.6 0.7 0.7)) "Undefined" "MultiplyWithRoot" null (0.0 0.0 0.0) null))
        (bind _output_get (set `self.AsArrowEquiped` _returnvalue))
        (`self.K2_AttachToComponent` _output_get (`/Game/RemoteGit/Player/BP_PlayerCharacterBossFight.SwordScene` (`self.As BP Player Character Boss Fight`)) "None" "SnapToTarget" "SnapToTarget" "KeepWorld" true)
        (`self.K2_AddActorLocalRotation` (`self.AsArrowEquiped`) (struct :`Pitch` 180.0 :`Yaw` 90.0) false false)
        (`self.K2_AddActorLocalOffset` _output_get (30.0 0.0 0.0) false false)))))

(event `EnhancedInput|/Game/RemoteGit/Player/EnhancedInputs/IA_MoveCamera`
  (params (ActionValue :type "Float (double-precision)") (ElapsedSeconds :type "Float (double-precision)") (TriggeredSeconds :type "Float (double-precision)") (InputAction :type "InputAction Object Reference" :default "/Game/RemoteGit/Player/EnhancedInputs/IA_MoveCamera.IA_MoveCamera"))
  (:`Triggered`
    (`/Game/RemoteGit/Player/BPC_CameraDrag.Receive Camera Override` (`self.BPC_CameraDrag`) (* ActionValue 0.25 (`/Game/RemoteGit/Player/Stats/PDATA_PlayerStats.CamerTurnSensivity` (`self.Player Stats`))))))

(event `EnhancedInput|/Game/RemoteGit/Player/EnhancedInputs/IA_MoveCameraEnabled`
  (params (ActionValue :type Boolean) (ElapsedSeconds :type "Float (double-precision)") (TriggeredSeconds :type "Float (double-precision)") (InputAction :type "InputAction Object Reference" :default "/Game/RemoteGit/Player/EnhancedInputs/IA_MoveCameraEnabled.IA_MoveCameraEnabled"))
  (bind _bpc_cameradrag (`self.BPC_CameraDrag`))
  (:`Triggered`
    (`/Game/RemoteGit/Player/BPC_CameraDrag.ToggleCameraInput` _bpc_cameradrag true :!label _label_5))
  (:`Started`
    (goto _label_5))
  (:`Canceled`
    (`/Game/RemoteGit/Player/BPC_CameraDrag.ToggleCameraInput` _bpc_cameradrag false :!label _label_6))
  (:`Completed`
    (goto _label_6)))

(event `/Game/RemoteGit/Player/AnimsBPs/BPI_Anims.PlayShake`
  (params (ShakeClass :type "LegacyCameraShake Class Reference"))
  (`LegacyCameraShake.StartLegacyCameraShake` (`GameplayStatics.GetPlayerCameraManager` 0) ShakeClass))

(fn `ChangeSelected weapon`
  (params (EquipedWepon :type "/Game/RemoteGit/Player/Weapons/E_Weapon Enum" :default "NewEnumerator0"))
  (bind _as_bp_player_character_boss_fight (`self.As BP Player Character Boss Fight`))
  (bind _output_get (set `self.EquipedWepon` EquipedWepon))
  (switch `/Game/RemoteGit/Player/Weapons/E_Weapon` _output_get
    (:`NewEnumerator0`
      (`/Game/RemoteGit/Player/BP_PlayerCharacterBossFight.DrawSwordToBow` _as_bp_player_character_boss_fight))
    (:`NewEnumerator1`
      (`/Game/RemoteGit/Player/BP_PlayerCharacterBossFight.DrawBowToSword` _as_bp_player_character_boss_fight)
      (set `/Game/RemoteGit/Player/AnimsBPs/AnimBP_Hero.BowEquiped` false (`self.AnimInstancePlayer`)))))

(fn `GetCameraFOV`
  (returns (`Field Of View` :type "Float (single-precision)"))
  (return (`CameraComponent.FieldOfView` (select `bool` (`self.CameraCenterRegistered`) :`false` (`/Game/RemoteGit/Player/BP_PlayerCharacterBossFight.Camera` (`self.As BP Player Character Boss Fight`)) :`true` (`/Game/RemoteGit/Player/BP_WorldCenter.Camera` (`self.World Center`))))))

(fn `InitArrows`
  (`/Game/RemoteGit/Widgets/Widget_Main.UpdateMaxArrows` (`self.Main Widget`) (`/Game/RemoteGit/Player/Stats/PDATA_PlayerStats.Max Arrow` (`self.Player Stats`)))
  (`self.Update Arrows` 0))

(fn `InputMovment`
  (params (InVec :type "Vector2D Structure"))
  (locals (Yaw :type "Float (double-precision)"))
  (bind (_returnvalue_roll _returnvalue_pitch _returnvalue_yaw) (`KismetMathLibrary.BreakRotator` (`self.GetControlRotation`)))
  (bind _as_bp_player_character_boss_fight (`self.As BP Player Character Boss Fight`))
  (bind (_x _y) (`KismetMathLibrary.BreakVector2D` (`local.InVec`)))
  (bind _returnvalue (`KismetMathLibrary.MakeRotator` 0.0 0.0 (`local.Yaw`)))
  (bind (_returnvalue_roll_2 _returnvalue_pitch_2 _returnvalue_yaw_2) (`KismetMathLibrary.BreakRotator` (`SceneComponent.K2_GetComponentRotation` (`/Game/RemoteGit/Player/BP_WorldCenter.SpringArm` (`self.World Center`)))))
  (`|ExecutionSequence`
    (:`then_0`
      (if (`self.CameraCenterRegistered`)
        (set `local.Yaw` _returnvalue_yaw_2)
        (else
          (set `local.Yaw` _returnvalue_yaw))))
    (:`then_1`
      (`Pawn.AddMovementInput` _as_bp_player_character_boss_fight (`KismetMathLibrary.GetRightVector` _returnvalue) _x false)
      (`Pawn.AddMovementInput` _as_bp_player_character_boss_fight (`KismetMathLibrary.GetForwardVector` _returnvalue) _y false))))

(fn `IsPlayerFalling`
  (returns (ReturnValue :type Boolean))
  (return (`NavMovementComponent.IsFalling` (`Character.CharacterMovement` (`self.As BP Player Character Boss Fight`)))))

(fn `MaxlifeChanged`
  (params (DeltaMaxHealth :type Integer))
  (bind _player_stats (`self.Player Stats`))
  (set `/Game/RemoteGit/Player/Stats/PDATA_PlayerStats.MaxHealth` (+ DeltaMaxHealth (`/Game/RemoteGit/Player/Stats/PDATA_PlayerStats.MaxHealth` _player_stats)) _player_stats)
  (`/Game/RemoteGit/Widgets/Widget_Main.RefreshMaxLife` (`self.Main Widget`))
  (`self.UpdateLife` 0))

(fn `Register New Camera`
  (params (NewViewAngle :type "Actor Object Reference"))
  (bind _world_center (`self.World Center`))
  (`self.SetViewTargetWithBlend` NewViewAngle 1.0 "VTBlend_EaseInOut" 1.0)
  (bind _asbp_world_center (cast `/Game/RemoteGit/Player/BP_WorldCenter` NewViewAngle)
    (:`then`
      (bind _output_get (set `self.World Center` _asbp_world_center))
      (`/Game/RemoteGit/Player/BP_WorldCenter.Register Player` _output_get (`self.As BP Player Character Boss Fight`))
      (set `self.CameraCenterRegistered` true)
      (`/Game/RemoteGit/Player/BPC_CameraDrag.Register New camera` (`self.BPC_CameraDrag`) (`/Game/RemoteGit/Player/BP_WorldCenter.Camera` (`self.World Center`))))
    (:`CastFailed`
      (set `self.CameraCenterRegistered` false)
      (`/Game/RemoteGit/Player/BPC_CameraDrag.Register New camera` (`self.BPC_CameraDrag`) (`/Game/RemoteGit/Player/BP_PlayerCharacterBossFight.Camera` (`self.As BP Player Character Boss Fight`)))
      (`/Engine/EditorBlueprintResources/StandardMacros.IsValid` _world_center
        (:`Is Valid`
          (`self.SetActorTickEnabled` _world_center false))))))

(fn `SetMaxArrows`
  (params (`Max Arrow` :type Integer))
  (bind _main_widget (`self.Main Widget`))
  (bind _output_get (set `/Game/RemoteGit/Player/Stats/PDATA_PlayerStats.Max Arrow` `Max Arrow` (`self.Player Stats`)))
  (`/Game/RemoteGit/Widgets/Widget_Main.UpdateArrows` _main_widget (`self.Arrows`))
  (`/Game/RemoteGit/Widgets/Widget_Main.UpdateMaxArrows` _main_widget _output_get))

(fn `Update Arrows`
  (params (Delta :type Integer))
  (bind _output_get (set `self.Arrows` (`KismetMathLibrary.Clamp` (+ (`self.Arrows`) Delta) 0 (`/Game/RemoteGit/Player/Stats/PDATA_PlayerStats.Max Arrow` (`self.Player Stats`)))))
  (`/Game/RemoteGit/Widgets/Widget_Main.UpdateArrows` (`self.Main Widget`) _output_get))

(fn `UpdateCameraFOV`
  (params (InFieldOfView :type "Float (single-precision)"))
  (if (`self.CameraCenterRegistered`)
    (`CameraComponent.SetFieldOfView` (`/Game/RemoteGit/Player/BP_WorldCenter.Camera` (`self.World Center`)) InFieldOfView)
    (else
      (`CameraComponent.SetFieldOfView` (`/Game/RemoteGit/Player/BP_PlayerCharacterBossFight.Camera` (`self.As BP Player Character Boss Fight`)) InFieldOfView))))

(fn `UpdateLife`
  (params (DeltaLife :type Integer))
  (bind _output_get (set `self.CurrentLife` (`KismetMathLibrary.Clamp` (+ DeltaLife (`self.CurrentLife`)) 0 (`/Game/RemoteGit/Player/Stats/PDATA_PlayerStats.MaxHealth` (`self.Player Stats`)))))
  (`/Game/RemoteGit/Widgets/Widget_Main.RefreshLife` (`self.Main Widget`))
  (`KismetSystemLibrary.PrintString` (`KismetStringLibrary.Conv_IntToString` _output_get)))

(fn `UserConstructionScript`)