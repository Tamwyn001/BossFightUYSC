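; Player controller component for the boss fight that lets input yaw the registered camera within a limit from player stats.
; Each tick it applies the clamped yaw, eases back toward the player, or snaps to look at the player when following.
; Releasing input starts a retriggerable delay before easing back.
; A gate holds that return after an arrow shot until the arrow arrives or input release reopens it.
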(event `self.ReceiveBeginPlay`
  (bind _asbp_play_controller_boss_fight (cast `/Game/RemoteGit/Player/BP_PlayControllerBossFight` (`self.GetOwner`)))
  (bind _output_get (set `self.As BP Play Controller Boss Fight` _asbp_play_controller_boss_fight))
  (set `self.Max Yaw Turn Camera` (`/Game/RemoteGit/Player/Stats/PDATA_PlayerStats.MaxYawTurnCamera` (`/Game/RemoteGit/Player/BP_PlayControllerBossFight.Player Stats` _output_get))))

(event `self.ReceiveTick`
  (params (DeltaSeconds :type "Float (single-precision)"))
  (bind _max_yaw_turn_camera (`self.Max Yaw Turn Camera`))
  (bind _returnvalue (`SceneComponent.K2_GetComponentRotation` (`self.Camera`)))
  (bind _returnvalue_location (`KismetMathLibrary.BreakTransform` (`Actor.GetTransform` (`self.Player Character`))))
  (bind _returnvalue_2 (`KismetMathLibrary.FindLookAtRotation` (`SceneComponent.K2_GetComponentLocation` (`self.Camera`)) _returnvalue_location))
  (if (and (not (`self.Transition to normal`)) (`self.Inputing`))
    (`SceneComponent.K2_SetRelativeRotation` (`self.Camera`) (`KismetMathLibrary.ComposeRotators` (`KismetMathLibrary.MakeRotator` 0.0 0.0 (`KismetMathLibrary.ClampAngle` (.yaw (`KismetMathLibrary.ComposeRotators` (`SceneComponent.RelativeRotation` (`self.Camera`)) (`KismetMathLibrary.MakeRotator` 0.0 0.0 (`self.CamneraOverwrite`)))) (* _max_yaw_turn_camera -1.0) _max_yaw_turn_camera)) (`self.Camera Base Rotation`)) false false)
    (elif (`self.Transition to normal`)
      (`SceneComponent.K2_SetWorldRotation` (`self.Camera`) (`KismetMathLibrary.RInterpTo` _returnvalue _returnvalue_2 DeltaSeconds 1.0) false false)
      (if (and (`KismetMathLibrary.NearlyEqual_FloatFloat` (.roll (`KismetMathLibrary.NormalizedDeltaRotator` _returnvalue _returnvalue_2)) 0.0 0.5) (`KismetMathLibrary.NearlyEqual_FloatFloat` (.pitch (`KismetMathLibrary.NormalizedDeltaRotator` _returnvalue _returnvalue_2)) 0.0 0.5) (`KismetMathLibrary.NearlyEqual_FloatFloat` (.yaw (`KismetMathLibrary.NormalizedDeltaRotator` _returnvalue _returnvalue_2)) 0.0 0.5))
        (set `self.Transition to normal` false)
        (set `self.CamneraOverwrite` 0.0))
      (else
        (`SceneComponent.K2_SetWorldRotation` (`self.Camera`) (`KismetMathLibrary.SelectRotator` _returnvalue _returnvalue_2 (or (not (`self.CameraFollowsPlayer`)) (`TimelineComponent.IsPlaying` (`/Game/RemoteGit/Player/BP_PlayControllerBossFight.CameraStartFollow` (`self.As BP Play Controller Boss Fight`))))) false false)))))

(event `Register New camera`
  (params (Camera :type "CameraComponent Object Reference"))
  (bind _output_get (set `self.Camera` Camera))
  (`self.SetComponentTickEnabled` true)
  (set `self.Player Character` (`GameplayStatics.GetPlayerCharacter` 0))
  (set `self.Camera Base Rotation` (`SceneComponent.RelativeRotation` _output_get)))

(event `ToggleCameraInput`
  (params (inputing :type Boolean))
  (bind _output_get (set `self.Inputing` inputing))
  (if _output_get
    (set `self.Transition to normal` false)
    (set `self.CameraFollowsPlayer` false)
    (else
      (set `self.CamneraOverwrite` 0.0)
      (`|ExecutionSequence` :!label _label
        (:`then_0`
          (`KismetSystemLibrary.RetriggerableDelay` 2.0)
          (`/Engine/EditorBlueprintResources/StandardMacros.Gate` true :!label _label_2
            (:`Exit`
              (set `self.Transition to normal` true)
              (set `self.CameraFollowsPlayer` true))))
        (:`then_1`
          (goto _label_2 :!via `Open`))))))

(event `Arrow Reached`
  (goto _label))

(event `Register Arrow shoot`
  (goto _label_2 :!via `Close`))

(fn `Receive Camera Override`
  (params (Yaw :type "Float (double-precision)"))
  (bind _output_get (set `self.CamneraOverwrite` Yaw))
  (`self.ToggleCameraInput` (not (== _output_get 0.0))))