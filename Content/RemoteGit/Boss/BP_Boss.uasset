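; BP_Boss is a flying boss character with a multi-phase health pool.
; Ten seconds after BeginPlay it calls NewAction, which spawns the first class in its waiting queue as an actor, passing itself as the boss.
; Damage lowers clamped health and broadcasts updates; depleting it advances the phase up to 3, announces the change and refills health.
; No death handling appears once health empties in phase 3.
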(event `NewAction`
  (`|SpawnActorFromClass` (`|GetArrayItem` (`self.WaintingCue`)) (`KismetMathLibrary.MakeTransform` (0.0 0.0 0.0)) "Undefined" "MultiplyWithRoot" null self null))

(event `self.ReceiveBeginPlay`
  (`CharacterMovementComponent.SetMovementMode` (`self.CharacterMovement`) "MOVE_Flying" 0)
  (`KismetSystemLibrary.Delay` 10.0)
  (`self.NewAction`))

(event `self.ReceiveAnyDamage`
  (params (Damage :type "Float (single-precision)") (DamageType :type "DamageType Object Reference") (InstigatedBy :type "Controller Object Reference") (DamageCauser :type "Actor Object Reference"))
  (set `self.CurrentHealth` (`KismetMathLibrary.FClamp` (- (`self.CurrentHealth`) Damage) 0.0 (`self.MaxHealth`)))
  (`self.HealthUpdate` (`self.CurrentHealth`))
  (if (== (`self.CurrentHealth`) 0.0)
    (switch `int` (`self.Current Phase`)
      (:`0`
        (bind _output_get (set `self.Current Phase` 1))
        (`self.PhaseChange` _output_get)
        (set `self.CurrentHealth` (`self.MaxHealth`)))
      (:`1`
        (bind _output_get_2 (set `self.Current Phase` 2))
        (`self.PhaseChange` _output_get_2)
        (set `self.CurrentHealth` (`self.MaxHealth`)))
      (:`2`
        (bind _output_get_3 (set `self.Current Phase` 3))
        (`self.PhaseChange` _output_get_3)
        (set `self.CurrentHealth` (`self.MaxHealth`))))))

(fn `UserConstructionScript`
  (set `self.CurrentHealth` (`self.MaxHealth`)))