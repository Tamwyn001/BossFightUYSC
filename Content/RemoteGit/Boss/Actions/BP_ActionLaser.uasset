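; Boss laser action that fires Niagara beams from both eyes, trailing the player.
; A looping timer traces from each eye toward below the player, scattering each target by its distance from the current beam point.
; Tick eases the beam ends, end effects and hit spheres toward those targets.
; The spheres damage actors on overlap and overlapping players on each timer pass; destruction removes the effects in two staggered pairs.
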(event `CalculateLocation`
  (bind _sphere (`self.Sphere`))
  (bind _returnvalue_location (`KismetMathLibrary.BreakTransform` (`self.GetTransform` (`GameplayStatics.GetPlayerCharacter` 0))))
  (bind _array (`|MakeArray` (`GameplayStatics.GetPlayerCharacter` 0) (`self.Boss`) :!type "Actor Object Reference"))
  (bind _returnvalue (- _returnvalue_location (0.0 0.0 100.0)))
  (bind _outhit (`KismetSystemLibrary.LineTraceSingle` (`SceneComponent.K2_GetComponentLocation` (`self.Niagara1`)) _returnvalue "TraceTypeQuery1" false _array))
  (bind _outhit_2 (`KismetSystemLibrary.LineTraceSingle` (`SceneComponent.K2_GetComponentLocation` (`self.Niagara`)) _returnvalue "TraceTypeQuery1" false _array))
  (bind (_bblockinghit _binitialoverlap _time _distance _location _impactpoint) (`GameplayStatics.BreakHitResult` _outhit))
  (set `self.Impact Point1` (+ _impactpoint (* (`KismetMathLibrary.MakeVector` (`KismetMathLibrary.RandomFloatInRange` -1.0 1.0) (`KismetMathLibrary.RandomFloatInRange` -1.0 1.0)) (`KismetMathLibrary.Vector_Distance` _impactpoint (`self.CurrentPoint1`)))))
  (bind (_bblockinghit_2 _binitialoverlap_2 _time_2 _distance_2 _location_2 _impactpoint_2) (`GameplayStatics.BreakHitResult` _outhit_2))
  (set `self.Impact Point2` (+ _impactpoint_2 (* (`KismetMathLibrary.MakeVector` (`KismetMathLibrary.RandomFloatInRange` -1.0 1.0) (`KismetMathLibrary.RandomFloatInRange` -1.0 1.0)) (`KismetMathLibrary.Vector_Distance` _impactpoint_2 (`self.CurrentPoint2`)))))
  (`ActorComponent.SetActive` _sphere true true)
  (`ActorComponent.SetActive` (`self.Sphere1`) true true)
  (`GameplayStatics.ApplyDamage` (`|GetArrayItem` (`PrimitiveComponent.GetOverlappingActors` (`self.Sphere1`) "/Game/RemoteGit/Player/BP_PlayerCharacterBossFight.BP_PlayerCharacterBossFight_C")) 4.0)
  (`GameplayStatics.ApplyDamage` (`|GetArrayItem` (`PrimitiveComponent.GetOverlappingActors` _sphere "/Game/RemoteGit/Player/BP_PlayerCharacterBossFight.BP_PlayerCharacterBossFight_C")) 4.0))

(event `self.ReceiveDestroyed`
  (`ActorComponent.K2_DestroyComponent` (`self.Niagara3`))
  (`ActorComponent.K2_DestroyComponent` (`self.Niagara1`))
  (`KismetSystemLibrary.Delay` 0.7)
  (`ActorComponent.K2_DestroyComponent` (`self.Niagara`))
  (`ActorComponent.K2_DestroyComponent` (`self.Niagara2`)))

(event `self.ReceiveBeginPlay`
  (bind _returnvalue (`NiagaraFunctionLibrary.SpawnSystemAttached` "/Game/RemoteGit/Niagara/PS_Laser.PS_Laser" (`Character.Mesh` (`self.Boss`)) "LEye" (0.0 0.0 0.0) (struct) "KeepRelativeOffset"))
  (set `self.Niagara` _returnvalue)
  (bind _returnvalue_2 (`NiagaraFunctionLibrary.SpawnSystemAttached` "/Game/RemoteGit/Niagara/PS_Laser.PS_Laser" (`Character.Mesh` (`self.Boss`)) "REye" (0.0 0.0 0.0) (struct) "KeepRelativeOffset"))
  (set `self.Niagara1` _returnvalue_2)
  (bind _returnvalue_3 (`NiagaraFunctionLibrary.SpawnSystemAtLocation` "/Game/RemoteGit/Niagara/NS_LaserEnd.NS_LaserEnd" (0.0 0.0 0.0) (struct) (1.0 1.0 1.0) false))
  (set `self.Niagara3` _returnvalue_3)
  (bind _returnvalue_4 (`NiagaraFunctionLibrary.SpawnSystemAtLocation` "/Game/RemoteGit/Niagara/NS_LaserEnd.NS_LaserEnd" (0.0 0.0 0.0) (struct) (1.0 1.0 1.0) false))
  (set `self.Niagara2` _returnvalue_4)
  (`KismetSystemLibrary.K2_SetTimerDelegate` (delegate `CalculateLocation`) 2.0 true))

(event `self.ReceiveTick`
  (params (DeltaSeconds :type "Float (single-precision)"))
  (bind _output_get (set `self.CurrentPoint1` (`KismetMathLibrary.VInterpTo` (`self.CurrentPoint1`) (`self.Impact Point1`) DeltaSeconds 1.0)))
  (bind _output_get_2 (set `self.CurrentPoint2` (`KismetMathLibrary.VInterpTo` (`self.CurrentPoint2`) (`self.Impact Point2`) DeltaSeconds 1.0)))
  (`NiagaraComponent.SetVariableVec3` (`self.Niagara1`) "user.BeamEnd" _output_get)
  (`NiagaraComponent.SetVariableVec3` (`self.Niagara`) "user.BeamEnd" _output_get_2)
  (`SceneComponent.K2_SetWorldLocation` (`self.Niagara3`) _output_get false false)
  (`SceneComponent.K2_SetWorldLocation` (`self.Sphere`) _output_get false false)
  (`SceneComponent.K2_SetWorldLocation` (`self.Niagara2`) _output_get_2 false false)
  (`SceneComponent.K2_SetWorldLocation` (`self.Sphere1`) _output_get_2 false false))

(event `self.Sphere.OnComponentBeginOverlap`
  (params (OverlappedComponent :type "PrimitiveComponent Object Reference") (OtherActor :type "Actor Object Reference") (OtherComp :type "PrimitiveComponent Object Reference") (OtherBodyIndex :type Integer) (bFromSweep :type Boolean) (SweepResult :type "HitResult Structure (by ref)"))
  (`GameplayStatics.ApplyDamage` OtherActor 4.0))

(event `self.Sphere1.OnComponentBeginOverlap`
  (params (OverlappedComponent :type "PrimitiveComponent Object Reference") (OtherActor :type "Actor Object Reference") (OtherComp :type "PrimitiveComponent Object Reference") (OtherBodyIndex :type Integer) (bFromSweep :type Boolean) (SweepResult :type "HitResult Structure (by ref)"))
  (`GameplayStatics.ApplyDamage` OtherActor 4.0))

(fn `UserConstructionScript`
  (`parent.UserConstructionScript`))