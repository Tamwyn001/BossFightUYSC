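; Destructible arena prop (jar or amphora) that spawns a drop when damaged and can be reset for reuse.
; Any damage spawns a BP_Dropable with its configured drop and a Niagara explosion tinted by the Color of the dynamic material created at BeginPlay.
; The mesh is then hidden without collision rather than destroyed, until Reset restores it.
; Randomize picks a random mesh and material instance.
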(event `Reset`
  (bind _staticmesh (`self.StaticMesh`))
  (`SceneComponent.SetVisibility` _staticmesh true false)
  (`PrimitiveComponent.SetCollisionEnabled` _staticmesh "QueryOnly"))

(event `self.ReceiveBeginPlay`
  (bind _staticmesh (`self.StaticMesh`))
  (bind _returnvalue (`PrimitiveComponent.CreateDynamicMaterialInstance` _staticmesh 0 (`PrimitiveComponent.GetMaterial` _staticmesh 0) "None"))
  (set `self.Material` _returnvalue))

(event `self.ReceiveAnyDamage`
  (params (Damage :type "Float (single-precision)") (DamageType :type "DamageType Object Reference") (InstigatedBy :type "Controller Object Reference") (DamageCauser :type "Actor Object Reference"))
  (bind _returnvalue_location (`KismetMathLibrary.BreakTransform` (`self.GetTransform`)))
  (bind _staticmesh (`self.StaticMesh`))
  (`|SpawnActorFromClass` "/Game/RemoteGit/Props/Dropable/BP_Dropable.BP_Dropable_C" (`KismetMathLibrary.MakeTransform` _returnvalue_location) "Undefined" "MultiplyWithRoot" null (`self.Implemented Drop`) null)
  (bind _returnvalue (`NiagaraFunctionLibrary.SpawnSystemAtLocation` "/Game/RemoteGit/Niagara/NS_ExplosionProp.NS_ExplosionProp" _returnvalue_location))
  (bind _returnvalue_2 (`MaterialInstanceDynamic.K2_GetVectorParameterValue` (`self.Material`) "Color"))
  (`FXSystemComponent.SetColorParameter` _returnvalue "user.color" _returnvalue_2)
  (`SceneComponent.SetVisibility` _staticmesh false false)
  (`PrimitiveComponent.SetCollisionEnabled` _staticmesh "NoCollision"))

(fn `Randomize`
  (bind _staticmesh (`self.StaticMesh`))
  (`StaticMeshComponent.SetStaticMesh` _staticmesh (`|GetArrayItem` (`|MakeArray` "/Game/RemoteGit/fbx/SM_ArenaProps_Jarre.SM_ArenaProps_Jarre" "/Game/RemoteGit/fbx/SM_ArenaProps_Amphore.SM_ArenaProps_Amphore" :!type "StaticMesh Object Reference") (`KismetMathLibrary.RandomIntegerInRange` 0 1)))
  (`PrimitiveComponent.SetMaterial` _staticmesh 0 (`|GetArrayItem` (`|MakeArray` "/Game/RemoteGit/fbx/M_Props_Inst.M_Props_Inst" "/Game/RemoteGit/fbx/M_Props_Inst1.M_Props_Inst1" "/Game/RemoteGit/fbx/M_Props_Inst2.M_Props_Inst2" "/Game/RemoteGit/fbx/M_Props_Inst3.M_Props_Inst3" "/Game/RemoteGit/fbx/M_Props_Inst4.M_Props_Inst4" :!type "MaterialInterface Object Reference") (`KismetMathLibrary.RandomIntegerInRange` 0 4))))

(fn `UserConstructionScript`)